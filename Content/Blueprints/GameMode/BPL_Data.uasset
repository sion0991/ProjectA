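; Blueprint function library for saving, loading and updating player and item data.
; SaveGame and LoadGame delegate to the player's AC_Status and AC_Inventory components, with inventory loaded before status.
; ItemUpdate refreshes a slot's saved inventory and equipment by replacing each item with its current BP_ItemTable row, matched by ItemIndex, then saves the slot.
; A generic table-row getter remains, named as currently unused.
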(fn GetItem현재사용X
  (params (TableInfo :type Data%20Table%20Row%20Handle%20Structure))
  (bind (_datatable _rowname) (Utilities|Struct|BreakDataTableRowHandle TableInfo))
  (Utilities|IsValid _datatable
    (:Is%20Valid
      (bind _returnvalue (Utilities|GetDataTableRow _datatable _rowname)
        (:then
          (return _returnvalue))))))

(fn SaveGame
  (params (Player :type Actor%20Object%20Reference))
  (LocalVariables|SetActor Player)
  (Default|SaveStatus (Actor|GetComponentbyClass (LocalVariables|GetActor) "/Game/Blueprints/State/AC_Status.AC_Status_C"))
  (Default|SaveInventory (Actor|GetComponentbyClass (LocalVariables|GetActor) "/Game/Blueprints/State/AC_Inventory.AC_Inventory_C")))

(fn LoadGame
  (params (Player :type Actor%20Object%20Reference))
  (LocalVariables|SetActor Player)
  (Default|LoadInventory (Actor|GetComponentbyClass (LocalVariables|GetActor) "/Game/Blueprints/State/AC_Inventory.AC_Inventory_C"))
  (Default|LoadStatus (Actor|GetComponentbyClass (LocalVariables|GetActor) "/Game/Blueprints/State/AC_Status.AC_Status_C")))

(fn ItemUpdate
  (params (Slot :type String))
  (bind _returnvalue (SaveGame|LoadGamefromSlot Slot))
  (bind _assave_inventory (Utilities|Casting|CastToSave_Inventory _returnvalue))
  (bind _output_get (LocalVariables|SetInventory _assave_inventory))
  (Utilities|FlowControl|Sequence
    (:then_0
      (for (_array_element _array_index) (Variables|/Game/Blueprints/Info/Save/Save_Inventory.Save_Inventory_C|GetInventory _output_get)
        (if (Utilities|Name|NotEqual(Name) (.itemindex _array_element) "None")
          (bind _returnvalue_2 (Utilities|GetDataTableRow "/Game/Blueprints/Info/Item/BP_ItemTable.BP_ItemTable" (.itemindex _array_element))
            (:then
              (Utilities|Array|SetArrayElem (Variables|/Game/Blueprints/Info/Save/Save_Inventory.Save_Inventory_C|GetInventory (LocalVariables|GetInventory)) _array_index _returnvalue_2))))))
    (:then_1
      (for (_array_element_2 _array_index_2) (Variables|/Game/Blueprints/Info/Save/Save_Inventory.Save_Inventory_C|GetEquipments _output_get)
        (if (Utilities|Name|NotEqual(Name) (.itemindex _array_element_2) "None")
          (bind _returnvalue_3 (Utilities|GetDataTableRow "/Game/Blueprints/Info/Item/BP_ItemTable.BP_ItemTable" (.itemindex _array_element_2))
            (:then
              (Utilities|Array|SetArrayElem (Variables|/Game/Blueprints/Info/Save/Save_Inventory.Save_Inventory_C|GetEquipments (LocalVariables|GetInventory)) _array_index_2 _returnvalue_3))))))
    (:then_2
      (SaveGame|SaveGametoSlot (LocalVariables|GetInventory) Slot)
      (return))))