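; BP_GM is a game mode Blueprint that spawns dropped items and holds slot-based save and load logic.
; DropAction spawns a BP_Item at the given transform and initializes it with the item data.
; LoadGame, marked as currently unused, restores stats, equipment and inventory to the player state, or creates a new save object when none exists.
; SaveGame is empty, and the async save call is disconnected.
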(event Custom|SaveGame
  (params (PlayerState :type BP%20Player%20State%20Object%20Reference))
  ;[1 1 1] 현재사용x
)

(event Custom|CreateSave
  ;[1 1 1] 현재사용x
  (bind _returnvalue (SaveGame|CreateSaveGameObject "/Game/Blueprints/Info/Save/BP_SaveGame.BP_SaveGame_C"))
  (bind _output_get (Variables|Default|SetSave _returnvalue))
  (Variables|/Game/Blueprints/Info/Save/BP_SaveGame.BP_SaveGame_C|SetSlotName _output_get (Variables|Default|GetSlot)))

(event Custom|LoadGame
  ;[1 1 1] 현재사용x
  (bind _returnvalue (SaveGame|DoesSaveGameExist (Variables|Default|GetSlot)))
  (if _returnvalue
    (if true
      (bind _returnvalue_2 (SaveGame|LoadGamefromSlot (Variables|Default|GetSlot)))
      (bind _asbp_save_game (Utilities|Casting|CastToBP_SaveGame _returnvalue_2))
      (bind _output_get (Variables|Default|SetSave _asbp_save_game))
      (bind _asbp_player (Utilities|Casting|CastToBP_Player (Game|GetPlayerCharacter 0)))
      (Default|SetInfo (Variables|/Game/Blueprints/Character/Player/BP_Player.BP_Player_C|GetAs%20BP%20Player%20State _asbp_player) (Variables|/Game/Blueprints/Info/Save/BP_SaveGame.BP_SaveGame_C|GetStat _output_get) (Variables|/Game/Blueprints/Info/Save/BP_SaveGame.BP_SaveGame_C|GetEquipItems _output_get) (Variables|/Game/Blueprints/Info/Save/BP_SaveGame.BP_SaveGame_C|GetInventory _output_get) (Variables|/Game/Blueprints/Info/Save/BP_SaveGame.BP_SaveGame_C|GetMaxInventoryIndex _output_get))
      (Development|PrintString "Load"))
    (else
      (bind _returnvalue_3 (SaveGame|CreateSaveGameObject "/Game/Blueprints/Info/Save/BP_SaveGame.BP_SaveGame_C"))
      (bind _output_get_2 (Variables|Default|SetSave _returnvalue_3))
      (Variables|/Game/Blueprints/Info/Save/BP_SaveGame.BP_SaveGame_C|SetSlotName _output_get_2 (Variables|Default|GetSlot)))))

(event Custom|DropAction
  (params (Item :type BP%20Item%20Struct%20Structure) (Transform :type Transform))
  (bind _returnvalue (Game|SpawnActorfromClass "/Game/Blueprints/Object/BP_Item.BP_Item_C" Transform "Undefined" 0 0))
  (Default|SpawnItem _returnvalue Item))

(event EventBeginPlay)

(fn ConstructionScript)