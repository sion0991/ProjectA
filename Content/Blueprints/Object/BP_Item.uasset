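; BP_Item is a world pickup that displays an item's mesh and pickup text, and goes into the player's inventory on interaction.
; SpawnItem applies the item info to the skeletal mesh and text widget; a test mode feeds it random or indexed BP_ItemTable rows at BeginPlay.
; Trigger overlaps toggle the widget and register the item as the player's interactable.
; Interacting in range adds it to ACInventory and destroys the actor.
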(event OnComponentBeginOverlap(Trigger)
  (params (OverlappedComponent :type Primitive%20Component%20Object%20Reference) (OtherActor :type Actor%20Object%20Reference) (OtherComp :type Primitive%20Component%20Object%20Reference) (OtherBodyIndex :type Integer) (bFromSweep :type Boolean) (SweepResult :type Hit%20Result%20Structure%20%28by%20ref%29))
  (bind _asbp_player (Utilities|Casting|CastToBP_Player OtherActor))
  (Rendering|SetVisibility (Variables|Default|GetWidget) true false)
  (Variables|Default|SetIsInRange true)
  (Variables|/Game/Blueprints/Character/Player/BP_Player.BP_Player_C|SetInterectableObject _asbp_player self))

(event OnComponentEndOverlap(Trigger)
  (params (OverlappedComponent :type Primitive%20Component%20Object%20Reference) (OtherActor :type Actor%20Object%20Reference) (OtherComp :type Primitive%20Component%20Object%20Reference) (OtherBodyIndex :type Integer))
  (bind _asbp_player (Utilities|Casting|CastToBP_Player OtherActor))
  (Rendering|SetVisibility (Variables|Default|GetWidget) false false)
  (Variables|Default|SetIsInRange false)
  (if (== (Variables|/Game/Blueprints/Character/Player/BP_Player.BP_Player_C|GetInterectableObject _asbp_player) self)
    (Variables|/Game/Blueprints/Character/Player/BP_Player.BP_Player_C|SetInterectableObject _asbp_player 0)))

(event Custom|SpawnItem
  (params (NewParam :type BP%20Item%20Struct%20Structure))
  (bind _output_get (Variables|Default|SetItemInfo NewParam))
  (Components|SkinnedMesh|SetSkinnedAssetandUpdate (Variables|Default|GetSkelMesh) (.meshpath _output_get) true)
  (bind _aswb_item_text (Utilities|Casting|CastToWB_ItemText (UserInterface|GetWidget (Variables|Default|GetWidget))))
  (Default|SetText _aswb_item_text (.pickuptext _output_get)))

(event Custom|TestSpawn
  (if (Variables|Default|GetIsRandom)
    (bind _returnvalue (Utilities|GetDataTableRow "/Game/Blueprints/Info/Item/BP_ItemTable.BP_ItemTable" (.OutItem (Utilities|Array|Random (Variables|Default|GetSpawnItems))))
      (:then
        (CallFunction|SpawnItem _returnvalue)))
    (else
      (bind _returnvalue_2 (Utilities|GetDataTableRow "/Game/Blueprints/Info/Item/BP_ItemTable.BP_ItemTable" (Utilities|Array|Get(acopy) (Variables|Default|GetSpawnItems) (Variables|Default|GetItemIndex)))
        (:then
          (CallFunction|SpawnItem _returnvalue_2))))))

(event EventInterectEvent
  (params (Player :type BPI%20Reciver%20Interface))
  (if (and (Collision|GetActorEnableCollision) (Variables|Default|GetIsInRange))
    (Default|AddItem (Variables|/Game/Blueprints/Character/Player/BP_Player.BP_Player_C|GetAC_Inventory (.AsBP%20Player (Utilities|Casting|CastToBP_Player Player))) (Variables|Default|GetItemInfo))
    (Actor|DestroyActor)))

(event EventBeginPlay
  (if (Variables|Default|GetIsTest)
    (CallFunction|TestSpawn)))

(fn ConstructionScript)

(fn ItemStats
  (if true
    (Variables|Default|SetItemInfo "")))