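; BP_EnterArea is an area trigger that moves linked meshes when the player enters it.
; On actor overlap with the first player's pawn, it calls OnMoveMesh on every MovableMeshes entry, provided the first element passes a comparison.
; A similar check on the first Monsters entry leads to no action, and a DestroyActor call is left unconnected, so the trigger can fire repeatedly.
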(event Collision|EventActorBeginOverlap
  (params (OtherActor :type Actor%20Object%20Reference))
  (bind _movablemeshes (Variables|Default|GetMovableMeshes))
  (if (== OtherActor (Game|Player|GetPlayerPawn 0))
    (Utilities|FlowControl|Sequence
      (:then_0
        (if (!= (Utilities|Array|Get(acopy) (Variables|Default|GetMonsters)) 0)
          _))
      (:then_1
        (if (!= (Utilities|Array|Get(acopy) _movablemeshes) 0)
          (for _array_element _movablemeshes
            (Default|OnMoveMesh _array_element)))))))

(fn ConstructionScript)