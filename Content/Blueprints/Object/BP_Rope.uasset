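; BP_Rope is an interactable rope that a player grabs and swings on.
; Interacting calls GrabRope on the player, and movement events push the physics-driven CableEnd with mass-independent force while its speed stays under a cap.
; GetEndSwingingForce and GetForce both return scaled CableEnd velocity as swing force.
; AddSwingingForce is an empty stub, and CableEnd2 only prints a debug message on cursor-over end.
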(event OnEndCursorOver(CableEnd2)
  (params (TouchedComponent :type Primitive%20Component%20Object%20Reference))
  (Development|PrintString "Hello"))

(event EventInterectEvent
  (params (Player :type BPI%20Reciver%20Interface))
  (Default|GrabRope Player self))

(event EventMoveForward
  (params (Value :type Float%20%28double-precision%29) (Direction :type Vector :default "0, 0, 0"))
  (if (< (Math|Vector|VectorLength (Transformation|GetComponentVelocity (Variables|Default|GetCableEnd))) 8e+02)
    (Physics|AddForce (Variables|Default|GetCableEnd) (* Direction (* Value 2e+02)) "None" true)))

(event EventMoveRight
  (params (Value :type Float%20%28double-precision%29) (Direction :type Vector :default "0, 0, 0"))
  (if (< (Math|Vector|VectorLength (Transformation|GetComponentVelocity (Variables|Default|GetCableEnd))) 8e+02)
    (Physics|AddForce (Variables|Default|GetCableEnd) (* Direction (* Value 2e+02)) "None" true)))

(fn ConstructionScript)

(fn AddSwingingForce
  (params (Force :type Vector)))

(fn GetEndSwingingForce
  (return (* (Transformation|GetComponentVelocity (Variables|Default|GetCableEnd)) 2.0)))

(fn GetForce
  (return (* (Transformation|GetComponentVelocity (Variables|Default|GetCableEnd)) 2.0)))