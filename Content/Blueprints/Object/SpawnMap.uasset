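; SpawnMap is an actor that builds a randomized MaxX by MaxY grid of two tile types.
; The construction script randomly stores 0 or 1 per cell in TileType, then adds an instance to one of two instanced static mesh components accordingly.
; Cell positions come from dividing the flat index by MaxY, scaled by TileSize in local space.
; Layout is re-rolled whenever construction runs, and the event graph has no logic.
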(event EventBeginPlay)

(event Collision|EventActorBeginOverlap
  (params (OtherActor :type Actor%20Object%20Reference)))

(event EventTick
  (params (DeltaSeconds :type Float%20%28single-precision%29)))

(fn ConstructionScript
  (bind _maxx (Variables|Default|GetMaxX))
  (bind _maxy (Variables|Default|GetMaxY))
  (bind _maxy_2 (Variables|Default|GetMaxY))
  (bind _tilesize (Variables|Default|GetTileSize))
  (bind _returnvalue (* _maxx _maxy))
  (bind _returnvalue_2 (- _returnvalue 1))
  (Utilities|Array|Resize (Variables|Default|GetTileType) _returnvalue_2)
  (for _index (range 0 _returnvalue_2)
    (Utilities|Array|SetArrayElem (Variables|Default|GetTileType) _index (Math|Random|RandomIntegerinRange 0 1))
    (if (== (Utilities|Array|Get(acopy) (Variables|Default|GetTileType) _index) 1)
      (Components|InstancedStaticMesh|AddInstance (Variables|Default|GetInstancedStaticMesh1) (Math|Conversions|ToTransform(Vector) (Math|Vector|MakeVector (Math|Conversions|ToFloat(Integer) (* (/ _index _maxy_2) _tilesize)) (Math|Conversions|ToFloat(Integer) (* (Math|Integer|%(Integer) _index _maxy_2) _tilesize)) 0.0)) false)
      (else
        (Components|InstancedStaticMesh|AddInstance (Variables|Default|GetInstancedStaticMesh) (Math|Conversions|ToTransform(Vector) (Math|Vector|MakeVector (Math|Conversions|ToFloat(Integer) (* (/ _index _maxy_2) _tilesize)) (Math|Conversions|ToFloat(Integer) (* (Math|Integer|%(Integer) _index _maxy_2) _tilesize)) 0.0)) false)))))