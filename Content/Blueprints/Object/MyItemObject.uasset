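; MyItemObject is a pickup item actor that displays a skeletal mesh and a text widget from its item info.
; On BeginPlay it casts its widget to CUW_ItemText and sets it to the item's pickup text.
; When IsTest is set, the construction script picks a random test spawn entry, looks up its row in the item data table, and copies that row's info and mesh onto the actor.
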(event EventBeginPlay
  (bind _ascuw_item_text (Utilities|Casting|CastToCUW_ItemText (UserInterface|GetWidget (Variables|Default|GetWidget))))
  (Class|UWItemText|SetText _ascuw_item_text (.pickuptext (Variables|Default|GetItemInfo))))

(event Collision|EventActorBeginOverlap
  (params (OtherActor :type Actor%20Object%20Reference)))

(fn ConstructionScript
  (if (Variables|Default|GetIsTest)
    (bind _returnvalue (Utilities|GetDataTableRow "/Game/Blueprints/Info/ItemTable.ItemTable" (.itemname (.OutItem (Utilities|Array|Random (Variables|Default|GetTestSpawnItemDatas)))))
      (:then
        (bind _output_get (Variables|Default|SetItemInfo _returnvalue))
        (Variables|/Script/Engine.SkeletalMeshComponent|SetSkeletalMeshAsset (Variables|Default|GetSkeletalMesh) (.skeletalmesh _output_get))))))