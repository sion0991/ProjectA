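; BPC_Item is a world item actor that shows a widget and registers as the player's interactable while overlapped.
; SpawnItem stores the item info, refreshes the skeletal mesh and clears the widget text.
; In test mode, BeginPlay spawns a random or indexed entry from the item DataTable.
; InteractEvent only checks controller, collision and range; pickup is unimplemented, with DestroyActor unwired and ItemStats empty.
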(event OnComponentBeginOverlap(Trigger)
  (params (OverlappedComponent :type Primitive%20Component%20Object%20Reference) (OtherActor :type Actor%20Object%20Reference) (OtherComp :type Primitive%20Component%20Object%20Reference) (OtherBodyIndex :type Integer) (bFromSweep :type Boolean) (SweepResult :type Hit%20Result%20Structure%20%28by%20ref%29))
  (bind _asmy_c_player (Utilities|Casting|CastToMyC_Player OtherActor))
  (Rendering|SetVisibility (Variables|Default|GetWidget) true false)
  (Variables|Default|SetIsInRange true)
  (Variables|/Script/ProjectA.C_Player|SetInteractableObject _asmy_c_player self))

(event OnComponentEndOverlap(Trigger)
  (params (OverlappedComponent :type Primitive%20Component%20Object%20Reference) (OtherActor :type Actor%20Object%20Reference) (OtherComp :type Primitive%20Component%20Object%20Reference) (OtherBodyIndex :type Integer))
  (bind _asmy_c_player (Utilities|Casting|CastToMyC_Player OtherActor))
  (Rendering|SetVisibility (Variables|Default|GetWidget) false false)
  (Variables|Default|SetIsInRange false)
  (if (== (Variables|/Script/ProjectA.C_Player|GetInteractableObject _asmy_c_player) self)
    (Variables|/Script/ProjectA.C_Player|SetInteractableObject _asmy_c_player 0)))

(event Custom|SpawnItem
  (params (ItemInfo :type ST%20Item%20Structure))
  (Variables|Default|SetItemInfo ItemInfo)
  (Components|SkinnedMesh|SetSkinnedAssetandUpdate (Variables|Default|GetSkelMesh) 0 true)
  (bind _aswb_item_text (Utilities|Casting|CastToWB_ItemText (UserInterface|GetWidget (Variables|Default|GetWidget))))
  (Default|SetText _aswb_item_text))

(event Custom|TestSpawn
  (if (Variables|Default|GetIsRandom)
    (bind _returnvalue (Utilities|GetDataTableRow "/Game/Blueprints/Info/ItemTable.ItemTable" (.OutItem (Utilities|Array|Random (Variables|Default|GetSpawnItems))))
      (:then
        (CallFunction|SpawnItem _returnvalue)))
    (else
      (bind _returnvalue_2 (Utilities|GetDataTableRow "/Game/Blueprints/Info/ItemTable.ItemTable" (Utilities|Array|Get(acopy) (Variables|Default|GetSpawnItems) (Variables|Default|GetItemIndex)))
        (:then
          (CallFunction|SpawnItem _returnvalue_2))))))

(event EventInteractEvent
  (params (Player :type C%20Player%20Object%20Reference))
  (Utilities|Casting|CastToPC_Player (Pawn|GetController Player))
  (if (and (Collision|GetActorEnableCollision) (Variables|Default|GetIsInRange))
    _))

(event EventBeginPlay
  (if (Variables|Default|GetIsTest)
    (CallFunction|TestSpawn)))

(fn ConstructionScript)

(fn ItemStats
  (if true
    _))