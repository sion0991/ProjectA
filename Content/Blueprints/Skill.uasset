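; Base Skill Blueprint that tracks the owning character and provides empty OnSkill and EndSkill functions as hooks for skill logic.
; On BeginPlay it casts its owner to BP_Character, stores it as SkillOwner and adds it to the Ignore list.
; IsIgnore searches that list to report whether a given target is excluded.
; Overlap, Tick and construction script do nothing here.
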(event EventBeginPlay
  (bind _asbp_character (Utilities|Casting|CastToBP_Character (Components|GetOwner)))
  (bind _output_get (Variables|Default|SetSkillOwner _asbp_character))
  (Utilities|Array|Add (Variables|Default|GetIgnore) _output_get))

(event Collision|EventActorBeginOverlap
  (params (OtherActor :type Actor%20Object%20Reference)))

(event EventTick
  (params (DeltaSeconds :type Float%20%28single-precision%29)))

(fn ConstructionScript)

(fn OnSkill)

(fn EndSkill)

(fn IsIgnore
  (params (Target :type BP%20Character%20Object%20Reference))
  (bind _array_element (Utilities|Array|ForEachLoopwithBreak (Variables|Default|GetIgnore) :!label _label)
    (:LoopBody
      (if (== _array_element Target)
        (goto _label Break)))
    (:Completed
      (return (== _array_element Target)))))