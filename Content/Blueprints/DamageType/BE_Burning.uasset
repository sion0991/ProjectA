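; Burning effect actor meant to deal damage over time to the actor it is attached to.
; On BeginPlay it binds DotDamage to a looping timer and sets its own lifespan from the Lifespan variable.
; DotDamage applies Damage to the attach parent, passing HitActor as the event instigator.
; The timer interval is set to zero, which in Unreal clears a timer instead of starting it.
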(event Custom|DotDamage
  (Game|Damage|ApplyDamage (Actor|GetAttachParentActor) (Variables|Default|GetDamage) (Variables|Default|GetHitActor) 0))

(event EventBeginPlay
  (|CallParentFunction)
  (Utilities|Time|SetTimerbyEvent (delegate Custom|DotDamage) 0.0 true)
  (Actor|SetLifeSpan (Variables|Default|GetLifespan)))

(fn ConstructionScript
  (|CallParentFunction))