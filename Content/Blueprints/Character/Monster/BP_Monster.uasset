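; BP_Monster is a monster character that reports sight and hearing to its AI blackboard and handles damage, stun and death.
; PawnSensing writes the target actor or noise location and switches the State key.
; Damage feeds ACStatus with triple headshots, updates the HP widget, and triggers ragdoll death.
; Stun uses a retriggerable delay before restoring attack and movement, while BeginPlay adjusts speed by mesh scale and calls an empty InitializeSkill.
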(event OnSeePawn(PawnSensing)
  (params (Pawn :type Pawn%20Object%20Reference))
  (if (== (Class|BlackboardComponent|GetValueasEnum (AI|GetBlackboard 0) (Utilities|Name|MakeLiteralName "State")) (Utilities|Enum|LiteralenumState_Monster "NewEnumerator0"))
    (AI|Components|Blackboard|SetValueasObject (AI|GetBlackboard 0) (Utilities|Name|MakeLiteralName "TargetActor") Pawn)
    (CallFunction|SetState "NewEnumerator1")
    (Development|PrintString "see")))

(event OnHearNoise(PawnSensing)
  (params (Instigator :type Pawn%20Object%20Reference) (Location :type Vector%20%28by%20ref%29 :default "0, 0, 0") (Volume :type Float%20%28single-precision%29))
  (AI|Components|Blackboard|SetValueasVector (AI|GetBlackboard 0) (Utilities|Name|MakeLiteralName "TargetLocation") Location)
  (CallFunction|SetState "NewEnumerator3")
  (Development|PrintString "noise"))

(event Custom|ResetAttackCooldown
  (Utilities|FlowControl|Delay (Math|Random|RandomFloatinRange 0.5 1.5))
  (Variables|Default|SetIsCanAct true))

(event Custom|OnMove)

(event EventBeginPlay
  (CallFunction|ParameterSetting))

(event EventDie
  (|CallParentFunction)
  (Class|AnimInstance|StopSlotAnimation (Components|SkeletalMesh|GetAnimInstance (Variables|Character|GetMesh)) 0.0 "None")
  (Rendering|SetVisibility (Variables|Default|GetWidget) false false)
  (CallFunction|SetState "NewEnumerator4")
  (Collision|SetCollisionEnabled (Variables|Default|GetCapsuleComponent) "NoCollision")
  (Physics|SetSimulatePhysics (Variables|Character|GetMesh) true))

(event Game|Damage|EventAnyDamage
  (params (Damage :type Float%20%28single-precision%29) (DamageType :type Damage%20Type%20Object%20Reference) (InstigatedBy :type Controller%20Object%20Reference) (DamageCauser :type Actor%20Object%20Reference))
  (if (not (== InstigatedBy (Pawn|GetController)))
    (CallFunction|SetHP Damage "None")))

(event Game|Damage|EventPointDamage
  (params (Damage :type Float%20%28single-precision%29) (DamageType :type Damage%20Type%20Object%20Reference) (HitLocation :type Vector :default "0, 0, 0") (HitNormal :type Vector :default "0, 0, 0") (HitComponent :type Primitive%20Component%20Object%20Reference) (BoneName :type Name :default "None") (ShotFromDirection :type Vector :default "0, 0, 0") (InstigatedBy :type Controller%20Object%20Reference) (DamageCauser :type Actor%20Object%20Reference) (HitInfo :type Hit%20Result%20Structure%20%28by%20ref%29))
  (CallFunction|SetHP Damage BoneName))

(event EventStun
  (params (Duration :type Float%20%28double-precision%29))
  (|CallParentFunction Duration)
  (Variables|Default|SetIsStun true)
  (Utilities|FlowControl|RetriggerableDelay Duration)
  (Variables|Default|SetIsStun false)
  (CallFunction|SetCanAttack true)
  (CallFunction|SetCanMove0 true))

(event EventTick
  (params (DeltaSeconds :type Float%20%28single-precision%29)))

(fn ConstructionScript
  (|CallParentFunction))

(fn SetState
  (params (State :type State_Monster%20Enum :default "NewEnumerator0"))
  (AI|Components|Blackboard|SetValueasEnum (AI|GetBlackboard 0) (Utilities|Name|MakeLiteralName "State") State))

(fn ParameterSetting
  (CallFunction|UpdateWidgetHP)
  (CallFunction|InitializeSpeed)
  (CallFunction|InitializeSkill))

(fn SetHP
  (params (Damage :type Float%20%28double-precision%29) (Bone :type Name))
  (bind _dead (Default|CalcCurrentHPIndex (Variables|Default|GetAC_Status) (select (Utilities|Name|Equal(Name) Bone "Head") (* Damage 3.0) Damage)))
  (CallFunction|UpdateWidgetHP)
  (if _dead
    (CallFunction|Die)))

(fn UpdateWidgetHP
  (bind _ac_status (Variables|Default|GetAC_Status))
  (bind _aswb_bear_hp (Utilities|Casting|CastToWB_BearHP (UserInterface|GetUserWidgetObject (Variables|Default|GetWidget))))
  (Default|SetHP _aswb_bear_hp (Variables|/Game/Blueprints/State/AC_Status.AC_Status_C|GetCurrentHP _ac_status) (.hp (Variables|/Game/Blueprints/State/AC_Status.AC_Status_C|GetStatus _ac_status))))

(fn InitializeSpeed
  (bind _charactermovement (Variables|Character|GetCharacterMovement))
  (Variables|/Script/Engine.CharacterMovementComponent|SetMaxWalkSpeed _charactermovement (+ (Variables|/Script/Engine.CharacterMovementComponent|GetMaxWalkSpeed _charactermovement) (* (Variables|/Script/Engine.CharacterMovementComponent|GetMaxWalkSpeed _charactermovement) (- (.x (Transformation|GetWorldScale (Variables|Character|GetMesh))) 1.0) 0.1))))

(fn SetCanMove0
  (params (CanMove :type Boolean))
  (AI|Components|Blackboard|SetValueasBool (AI|GetBlackboard 0) (Utilities|Name|MakeLiteralName "CanMove") CanMove))

(fn GetTargetwhenValid
  (bind _returnvalue (AI|GetBlackboard 0))
  (bind _returnvalue_2 (Utilities|Name|MakeLiteralName "TargetActor"))
  (bind _returnvalue_3 (AI|Components|Blackboard|GetValueasObject _returnvalue _returnvalue_2))
  (Utilities|IsValid _returnvalue_3
    (:Is%20Valid
      (bind _as액터 (Utilities|Casting|CastToActor _returnvalue_3))
      (return _as액터))))

(fn GetState
  (params (Key :type Name))
  (return (Utilities|Enum|ByteToEnumState_Monster (Class|BlackboardComponent|GetValueasEnum (AI|GetBlackboard 0) Key))))

(fn InitializeSkill)

(fn GetCanAttack
  (return (Variables|Default|GetIsCanAct)))

(fn SetCanAttack
  (params (CanAttack :type Boolean))
  (Variables|Default|SetIsCanAct CanAttack))