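; BP_Warrior_2 is a warrior monster character that stands still until its OnMove event sends it after the player.
; BeginPlay stops active movement and caches the mesh's ABP_Warrior anim instance.
; OnMove sets IsFight on that anim Blueprint and runs AIMoveTo toward player character 0.
; Tick is empty, and a node chain to rotate the warrior toward the player is left unconnected.
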(event EventTick
  (params (DeltaSeconds :type Float%20%28single-precision%29)))

(event EventBeginPlay
  (Class|NavMovementComponent|StopActiveMovement (Variables|Character|GetCharacterMovement))
  (bind _asabp_warrior (Utilities|Casting|CastToABP_Warrior (Components|SkeletalMesh|GetAnimInstance (Variables|Character|GetMesh))))
  (Variables|Default|SetAs%20ABP%20Warrior _asabp_warrior))

(event EventOnMove
  (Variables|/Game/Blueprints/Character/Monster/Warrior/ABP_Warrior.ABP_Warrior_C|SetIsFight (Variables|Default|GetAs%20ABP%20Warrior) true)
  (AI|AIMoveTo self "0, 0, 0" (Game|GetPlayerCharacter 0) 5.0 false))

(fn ConstructionScript)