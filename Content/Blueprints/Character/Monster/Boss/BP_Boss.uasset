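; Boss monster Blueprint that extends its parent's parry and death behavior and sets up the boss's attack skills.
; InitializeSkill looks up AttackTable rows keyed by the boss Name plus an index and feeds each found row to ACAttack.SkillSetting.
; Being parried plays a dedicated parried montage after the parent handling.
; Death runs the parent logic, then spawns a random handful of BP_Item drops at the mesh's transform.
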(event EventBeginPlay
  (|CallParentFunction))

(event EventParried
  (params (Duration :type Float%20%28double-precision%29))
  (|CallParentFunction Duration)
  (Animation|PlayAnimMontage "/Game/Asset/BossyEnemy/Animations/RootMotion/Boss_Parried_RM_Montage.Boss_Parried_RM_Montage" 1.0 "None"))

(event EventDie
  (|CallParentFunction)
  (for _index (range 0 (Math|Random|RandomIntegerinRange 0 3))
    (Game|SpawnActorfromClass "/Game/Blueprints/Object/BP_Item.BP_Item_C" (Transformation|GetWorldTransform (Variables|Character|GetMesh)) "Undefined" 0 0)))

(fn ConstructionScript
  (|CallParentFunction))

(fn InitializeSkill
  (for _index (range 0 5)
    (bind _returnvalue (Utilities|GetDataTableRow "/Game/Blueprints/Character/Monster/AttackTable.AttackTable" (Utilities|String|StringToName (Utilities|String|Append (Variables|Default|GetName) (Utilities|String|ToString(Integer) _index))))
      (:then
        (Default|SkillSetting (Variables|Default|GetAC_Attack) _returnvalue)))))