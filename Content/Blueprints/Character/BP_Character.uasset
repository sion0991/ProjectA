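; Character Blueprint providing combat reactions, paired finisher executions and entry into wall climbing.
; Finishers pick a random ACAttack FinishData entry, snap the attacker's capsule to its distance from the target, and play matched attacker/victim montages with yaw-only facing.
; ClimbWall turns into the hit surface, zeroes velocity, switches to Flying and blocks actions.
; Parried forwards to Stun, which, like Die, is an empty stub.
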(event Custom|Parried
  (params (Duration :type Float%20%28double-precision%29))
  (CallFunction|Stun Duration))

(event Custom|Stun
  (params (Duration :type Float%20%28double-precision%29)))

(event Custom|Die)

(event EventClimbWall
  (bind _charactermovement (Variables|Character|GetCharacterMovement))
  (Transformation|SetActorRotation (Math|Rotator|MakeRotator 0.0 0.0 (+ (.yaw (Math|Conversions|RotationFromXVector (.normal (Variables|Default|GetHitResult)))) 1.8e+02)))
  (Variables|Default|SetState "NewEnumerator1")
  (Variables|/Script/Engine.MovementComponent|SetVelocity _charactermovement "0, 0, 0")
  (Pawn|Components|CharacterMovement|SetMovementMode _charactermovement "MOVE_Flying" 0)
  (Variables|/Script/Engine.CharacterMovementComponent|SetbOrientRotationToMovement _charactermovement false)
  (Variables|/Script/Engine.CharacterMovementComponent|SetbUseControllerDesiredRotation _charactermovement false)
  (Variables|Default|SetIsCanAct false))

(event EventExecuteFinisherVictim
  (params (Target :type Character%20Object%20Reference) (FinisherIndex :type Integer))
  (Animation|Montage|MontagePlay (Components|SkeletalMesh|GetAnimInstance (Variables|/Script/Engine.Character|GetMesh Target)) (.victimmontage (Utilities|Array|Get(acopy) (Variables|/Game/Blueprints/State/AC_Attack.AC_Attack_C|GetFinishData (Variables|Default|GetAC_Attack)) FinisherIndex)) 1.0 "MontageLength" 0.0 true)
  (Transformation|SetActorRotation (Variables|Default|GetTarget) (Math|Rotator|MakeRotator 0.0 0.0 (.Yaw (Math|Rotator|BreakRotator (Math|Rotator|FindLookatRotation (Transformation|GetActorLocation (Variables|Default|GetTarget)) (Transformation|GetActorLocation)))))))

(event EventFinishable
  (bind _returnvalue (Transformation|GetActorLocation))
  (bind _ac_attack (Variables|Default|GetAC_Attack))
  (bind _target (Variables|Default|GetTarget))
  (bind _returnvalue_2 (Transformation|GetActorLocation _target))
  (bind _finishdata (Variables|/Game/Blueprints/State/AC_Attack.AC_Attack_C|GetFinishData _ac_attack))
  (bind _returnvalue_3 (Math|Rotator|FindLookatRotation _returnvalue _returnvalue_2))
  (bind _yaw (Math|Rotator|BreakRotator _returnvalue_3))
  (bind _returnvalue_4 (Math|Rotator|MakeRotator 0.0 0.0 _yaw))
  (if (Variables|Default|GetIsCanAct)
    (Utilities|IsValid (Variables|Default|GetTarget)
      (:Is%20Valid
        (Variables|Default|SetIsCanAct false)
        (bind _output_get (Variables|Default|SetFinish%20Index (Math|Random|RandomInteger (Utilities|Array|Length _finishdata))))
        (Animation|Montage|MontagePlay (Components|SkeletalMesh|GetAnimInstance (Variables|Character|GetMesh)) (.attackermontage (Utilities|Array|Get(acopy) _finishdata _output_get)) 1.0 "MontageLength" 0.0 true)
        (Transformation|SetWorldTransform (Variables|Collision|GetCapsuleComponent) (Math|Transform|MakeTransform (+ _returnvalue_2 (* (Math|Rotator|GetRotationXVector _returnvalue_4) (.distance (Utilities|Array|Get(acopy) _finishdata _output_get)))) _returnvalue_4 "1.000000,1.000000,1.000000") false false)
        (CallFunction|ExecuteFinisherVictim (Variables|Default|GetTarget) (Variables|Default|GetFinish%20Index))))))

(fn ConstructionScript)