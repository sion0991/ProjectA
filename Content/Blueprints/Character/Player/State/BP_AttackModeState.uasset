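; Player state for attack mode, which handles movement input and places equipped weapons in their active sockets.
; EnterState, when ItemSet is true, attaches main and sub weapons from the inventory using each item's socket and transform.
; Equip changes swap or clear the component's mesh and re-attach it likewise.
; One item type in the off-hand (sub slot or non-RWeapon component) instead uses the LeftWeapon socket with a hard-coded transform.
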(fn InputMoveForward
  (params (Value :type Float%20%28double-precision%29) (Direction :type Vector :default "0, 0, 0"))
  (Pawn|Input|AddMovementInput (Variables|Default|GetPlayerRef) Direction Value false)
  (Default|SetInputFwd (Variables|/Game/Blueprints/Character/Player/BP_Player.BP_Player_C|GetAs%20BPI%20Anim (Variables|Default|GetPlayerRef)) Value))

(fn InputChangeEquip
  (params (Item :type BP%20Item%20Struct%20Structure) (EquipComp :type Skeletal%20Mesh%20Component%20Object%20Reference))
  (bind (_itemtype _meshpath) (Utilities|Struct|BreakBP_ItemStruct Item))
  (bind (_meshpath_2 _atransform _asocket) (Utilities|Struct|BreakBP_ItemStruct Item))
  (|CallParentFunction "" 0)
  (Utilities|IsValid _meshpath
    (:Is%20Valid
      (if (Utilities|Enum|NotEqual(Enum) _itemtype "NewEnumerator16")
        (Components|SkinnedMesh|SetSkinnedAssetandUpdate EquipComp _meshpath_2 true :!label _label)
        (Transformation|AttachComponentToComponent EquipComp (Transformation|GetAttachParent EquipComp) _asocket "SnapToTarget" "SnapToTarget" "SnapToTarget" true)
        (Transformation|SetRelativeTransform EquipComp _atransform false false)
        (elif (Utilities|Enum|Equal(Enum) (Utilities|GetObjectName EquipComp) "RWeapon")
          (goto _label)
          (else
            (Components|SkinnedMesh|SetSkinnedAssetandUpdate EquipComp (.MeshPath (Utilities|Struct|BreakBP_ItemStruct Item)) true)
            (Transformation|AttachComponentToComponent EquipComp (Transformation|GetAttachParent EquipComp) "LeftWeapon" "SnapToTarget" "SnapToTarget" "SnapToTarget" true)
            (Transformation|SetRelativeTransform EquipComp (Math|Transform|MakeTransform "1.400000, 0,10.000000" "190.000000, 0, 0") false false)))))
    (:Is%20Not%20Valid
      (Components|SkinnedMesh|SetSkinnedAssetandUpdate EquipComp 0 true))))

(fn InputMoveRight
  (params (Value :type Float%20%28double-precision%29) (Direction :type Vector :default "0, 0, 0"))
  (Pawn|Input|AddMovementInput (Variables|Default|GetPlayerRef) Direction Value false)
  (Default|SetInputRight (Variables|/Game/Blueprints/Character/Player/BP_Player.BP_Player_C|GetAs%20BPI%20Anim (Variables|Default|GetPlayerRef)) Value))

(fn EnterState
  (params (Player :type BP%20Player%20Object%20Reference) (ItemSet :type Boolean))
  (bind _playerref (Variables|Default|GetPlayerRef))
  (bind _playerref_2 (Variables|Default|GetPlayerRef))
  (bind _playerref_3 (Variables|Default|GetPlayerRef))
  (bind _ac_inventory (Variables|/Game/Blueprints/Character/Player/BP_Player.BP_Player_C|GetAC_Inventory _playerref))
  (bind _ac_inventory_2 (Variables|/Game/Blueprints/Character/Player/BP_Player.BP_Player_C|GetAC_Inventory _playerref_3))
  (bind _mainweapon (Variables|/Game/Blueprints/Character/Player/BP_Player.BP_Player_C|GetMainWeapon _playerref_3))
  (bind _subweapon (Variables|/Game/Blueprints/Character/Player/BP_Player.BP_Player_C|GetSubWeapon _playerref_2))
  (bind _subweapon_2 (Variables|/Game/Blueprints/Character/Player/BP_Player.BP_Player_C|GetSubWeapon _playerref_2))
  (bind _newparam1 (Default|GetEquipItem _ac_inventory 1))
  (bind _newparam1_2 (Default|GetEquipItem _ac_inventory_2))
  (bind (_itemindex _itemtype _meshpath _atransform _bsocket _asocket) (Utilities|Struct|BreakBP_ItemStruct _newparam1))
  (bind (_itemindex_2 _meshpath_2 _atransform_2 _bsocket_2 _asocket_2) (Utilities|Struct|BreakBP_ItemStruct _newparam1_2))
  (|CallParentFunction Player false)
  (if ItemSet
    (Utilities|FlowControl|Sequence
      (:then_0
        (if (Utilities|Name|NotEqual(Name) _itemindex_2 "None")
          (Transformation|AttachComponentToComponent _mainweapon (Variables|/Script/Engine.Character|GetMesh _playerref_3) _asocket_2 "SnapToTarget" "SnapToTarget" "SnapToTarget" true)
          (Transformation|SetRelativeTransform _mainweapon _atransform_2 false false)))
      (:then_1
        (if (Utilities|Name|NotEqual(Name) _itemindex "None")
          (if (Utilities|Enum|Equal(Enum) _itemtype "NewEnumerator16")
            (Transformation|AttachComponentToComponent _subweapon (Variables|/Script/Engine.Character|GetMesh _playerref_2) "LeftWeapon" "SnapToTarget" "SnapToTarget" "SnapToTarget" true)
            (Transformation|SetRelativeTransform _subweapon (Math|Transform|MakeTransform "1.400000, 0,10.000000" (Math|Rotator|MakeRotator 0.0 1.9e+02 0.0)) false false)
            (else
              (Transformation|AttachComponentToComponent _subweapon_2 (Variables|/Script/Engine.Character|GetMesh _playerref_2) _asocket "SnapToTarget" "SnapToTarget" "SnapToTarget" true)
              (Transformation|SetRelativeTransform _subweapon_2 _atransform false false))))))))

(fn ExitState
  (|CallParentFunction))

(fn UpdateState
  (|CallParentFunction))