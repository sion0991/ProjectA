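; Player state for hanging on a rope, part of the player character's state set with enter, update, exit and input overrides.
; Forward and right input both drive MoveForward on the player's Riding reference and feed the anim interface's right input.
; On enter, it optionally moves main and sub weapons to the UnEquip socket using inventory transforms.
; Equipment changes set the new mesh on the given component and attach it at the item's B socket and transform.
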(fn InputMoveForward
  (params (Value :type Float%20%28double-precision%29) (Direction :type Vector :default "0, 0, 0"))
  (Default|MoveForward (Variables|/Game/Blueprints/Character/Player/BP_Player.BP_Player_C|GetRiding (Variables|Default|GetPlayerRef)) Value Direction)
  (Default|SetInputRight (Variables|/Game/Blueprints/Character/Player/BP_Player.BP_Player_C|GetAs%20BPI%20Anim (Variables|Default|GetPlayerRef)) Value))

(fn InputChangeEquip
  (params (Item :type BP%20Item%20Struct%20Structure) (EquipComp :type Skeletal%20Mesh%20Component%20Object%20Reference))
  (bind (_meshpath _btransform _bsocket) (Utilities|Struct|BreakBP_ItemStruct Item))
  (|CallParentFunction "" 0)
  (if (!= EquipComp 0)
    (Components|SkinnedMesh|SetSkinnedAssetandUpdate EquipComp _meshpath true)
    (Transformation|SetRelativeTransform EquipComp _btransform false false)
    (Transformation|AttachComponentToComponent EquipComp (Transformation|GetAttachParent EquipComp) _bsocket "KeepRelative" "KeepRelative" "KeepRelative" true)))

(fn InputMoveRight
  (params (Value :type Float%20%28double-precision%29) (Direction :type Vector :default "0, 0, 0"))
  (Default|MoveForward (Variables|/Game/Blueprints/Character/Player/BP_Player.BP_Player_C|GetRiding (Variables|Default|GetPlayerRef)) Value Direction)
  (Default|SetInputRight (Variables|/Game/Blueprints/Character/Player/BP_Player.BP_Player_C|GetAs%20BPI%20Anim (Variables|Default|GetPlayerRef)) Value))

(fn EnterState
  (params (Player :type BP%20Player%20Object%20Reference) (ItemSet :type Boolean))
  (bind _playerref (Variables|Default|GetPlayerRef))
  (bind _playerref_2 (Variables|Default|GetPlayerRef))
  (bind _mainweapon (Variables|/Game/Blueprints/Character/Player/BP_Player.BP_Player_C|GetMainWeapon _playerref_2))
  (bind _subweapon (Variables|/Game/Blueprints/Character/Player/BP_Player.BP_Player_C|GetSubWeapon _playerref))
  (|CallParentFunction Player false)
  (if ItemSet
    (Utilities|FlowControl|Sequence
      (:then_0
        (Transformation|AttachComponentToComponent _mainweapon (Variables|/Script/Engine.Character|GetMesh _playerref_2) "UnEquip" "SnapToTarget" "SnapToTarget" "SnapToTarget" true)
        (Transformation|SetRelativeTransform _mainweapon (.BTransform (Utilities|Struct|BreakBP_ItemStruct (Default|GetEquipItem (Variables|/Game/Blueprints/Character/Player/BP_Player.BP_Player_C|GetAC_Inventory _playerref_2)))) false false))
      (:then_1
        (Transformation|AttachComponentToComponent _subweapon (Variables|/Script/Engine.Character|GetMesh _playerref) "UnEquip" "SnapToTarget" "SnapToTarget" "SnapToTarget" true)
        (Transformation|SetRelativeTransform _subweapon (.BTransform (Utilities|Struct|BreakBP_ItemStruct (Default|GetEquipItem (Variables|/Game/Blueprints/Character/Player/BP_Player.BP_Player_C|GetAC_Inventory _playerref) 1))) false false)))))

(fn ExitState
  (|CallParentFunction))

(fn UpdateState
  (|CallParentFunction))