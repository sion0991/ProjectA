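; BP_PlayerState is a player state that stores the player's stats, equipment array and inventory, with getters and a setter to transfer them.
; Events drop, equip, unequip and consume items by moving entries between the arrays.
; Equipping picks the slot from item type, with foot armor choosing between two indices.
; An event graph note marks logic as currently unused, and the Stat assignments have no input.
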(event Custom|DropItem
  (params (NewParam :type Integer))
  ;[1 1 1] 현재사용X
  (Utilities|Array|RemoveIndex (Variables|Default|GetInventory) NewParam))

(event Custom|DurationItem
  (params (NewParam2 :type BP%20Item%20Struct%20Structure) (NewParam :type Integer))
  ;[1 1 1] 현재사용X
  (Utilities|FlowControl|Sequence
    (:then_1
      (Utilities|Array|RemoveIndex (Variables|Default|GetInventory) NewParam))))

(event Custom|TakeOffItem
  (params (NewParam2 :type BP%20Item%20Struct%20Structure) (NewParam :type Integer))
  ;[1 1 1] 현재사용X
  (Variables|Default|SetStat "")
  (Utilities|Array|Add (Variables|Default|GetInventory) NewParam2)
  (Utilities|Array|RemoveIndex (Variables|Default|GetEquipItems) NewParam))

(event Custom|EquipItem
  (params (Item :type BP%20Item%20Struct%20Structure) (NewParam :type Integer))
  ;[1 1 1] 현재사용X
  (Variables|Default|SetStat "")
  (Utilities|Array|SetArrayElem :TargetArray (Variables|Default|GetEquipItems) :Index (Utilities|Select :Index (.ItemType (Utilities|Struct|BreakBP_ItemStruct Item)) :NewEnumerator0 0 :NewEnumerator1 0 :NewEnumerator4 0 :NewEnumerator2 0 :NewEnumerator10 0 :NewEnumerator12 1 :NewEnumerator16 0 :NewEnumerator9 2 :NewEnumerator3 3 :NewEnumerator5 4 :NewEnumerator6 5 :NewEnumerator7 (Math|Integer|SelectInt 7 6 (Utilities|Array|IsValidIndex (Variables|Default|GetEquipItems) 6)) :NewEnumerator8 0 :NewEnumerator11 0 :NewEnumerator15 0))
  (Utilities|Array|RemoveIndex (Variables|Default|GetInventory) NewParam))

(fn ConstructionScript)

(fn GetItem
  (params (NewParam1 :type Integer))
  (return (Utilities|Array|Get(acopy) (Variables|Default|GetInventory) NewParam1)))

(fn GetInfo
  (return (Variables|Default|GetStat) (Variables|Default|GetEquipItems) (Variables|Default|GetInventory) (Variables|Default|GetMaxInventoryIndex)))

(fn SetInfo
  (params (Stat :type ST%20Status%20Structure) (Equips :type Array%20of%20BP%20Item%20Struct%20Structures) (Inventory :type Array%20of%20BP%20Item%20Struct%20Structures) (InventoryIndex :type Integer))
  (Variables|Default|SetStat Stat)
  (Variables|Default|SetEquipItems Equips)
  (Variables|Default|SetInventory Inventory)
  (Variables|Default|SetMaxInventoryIndex InventoryIndex))