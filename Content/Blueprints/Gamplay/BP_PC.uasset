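; BP_PC is a player controller that relays movement and jump input to the possessed pawn through the BPI_Reciver interface.
; On possess it stores the pawn as that interface, then after a short delay calls LoadInformation on it and caches the BP_HUD reference.
; Axis and jump events call the interface's input functions, keeping the controller independent of the pawn class.
; A BP_PlayerState cast is present but never executed.
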(event EventPossess
  (params (PossessedPawn :type Pawn%20Object%20Reference))
  (bind _asbpi_reciver (Utilities|Casting|CastToBPI_Reciver PossessedPawn))
  (bind _output_get (Variables|Default|SetPossessedPawn _asbpi_reciver))
  (Utilities|FlowControl|Delay 0.5)
  (Default|LoadInformation _output_get)
  (bind _asbp_hud (Utilities|Casting|CastToBP_HUD (HUD|GetHUD)))
  (Variables|Default|SetHUD _asbp_hud))

(event Input|ActionEvents|InputActionJump
  (params (Key :type Key%20Structure :default "None"))
  (:Pressed
    (Default|InputJump (Variables|Default|GetPossessedPawn))))

(event Input|AxisEvents|InputAxisMoveForward
  (params (AxisValue :type Float%20%28single-precision%29))
  (Default|InputMoveForward (Variables|Default|GetPossessedPawn) AxisValue))

(event Input|AxisEvents|InputAxisMoveRight
  (params (AxisValue :type Float%20%28single-precision%29))
  (Default|InputMoveRight (Variables|Default|GetPossessedPawn) AxisValue))

(fn ConstructionScript)