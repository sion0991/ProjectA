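; Player controller for the lobby that handles server selection, then character selection, and opens the TopDown level.
; It shows the Main_Lobby widget at start; confirming a chosen server removes it and zooms the LobbyPawn to the character stage.
; A shared ClickObject tracks the current pick so the previous server or character can be deselected.
; Double-clicking a character loads the level, detected by a click counter reset through a short retriggerable delay.
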(event Custom|ResetClickCount
  (Utilities|FlowControl|RetriggerableDelay 0.2)
  (Variables|Default|SetClickCount 0))

(event EventBeginPlay
  (bind _returnvalue (UserInterface|CreateWidget "/Game/Blueprints/UI/Main_Lobby.Main_Lobby_C" self))
  (bind _output_get (Variables|Default|SetWB_SelectServer _returnvalue))
  (UserInterface|Viewport|AddtoViewport _output_get 0))

(fn ConstructionScript)

(fn SelectServer
  (params (Server :type Lobby%20Server%20Object%20Reference))
  (Utilities|IsValid (Variables|Default|GetClickObject)
    (:Is%20Valid
      (bind _aslobby_server (Utilities|Casting|CastToLobby_Server (Variables|Default|GetClickObject)))
      (Default|SetCheckServer _aslobby_server "Hidden"))
    (:Is%20Not%20Valid
      _))
  (Variables|Default|SetClickObject Server))

(fn OnWBSelectCharacter
  (Utilities|IsValid (Variables|Default|GetClickObject)
    (:Is%20Valid
      (Widget|RemovefromParent (Variables|Default|GetWB_SelectServer))
      (Variables|Default|SetClickObject 0)
      (bind _aslobby_pawn (Utilities|Casting|CastToLobbyPawn (Pawn|GetControlledPawn)))
      (Default|ZoominCharacterLevel _aslobby_pawn))
    (:Is%20Not%20Valid
      (Development|PrintString "서버를 선택해야 접속할 수 있습니다."))))

(fn SelectCharacter
  (params (SelectChar :type BP%20Select%20Character%20Object%20Reference))
  (bind _isdoubleclick (CallFunction|MouseClick SelectChar))
  (if _isdoubleclick
    (Game|OpenLevel(byObjectReference) "/Game/TopDown/Maps/TopDown.TopDown")
    (else
      (Utilities|IsValid (Variables|Default|GetClickObject)
        (:Is%20Valid
          (bind _asbp_select_character (Utilities|Casting|CastToBP_SelectCharacter (Variables|Default|GetClickObject)))
          (Default|Selected _asbp_select_character false))
        (:Is%20Not%20Valid
          _))
      (Variables|Default|SetClickObject SelectChar))))

(fn MouseClick
  (params (ClickActor :type Object%20Object%20Reference))
  (Math|Integer|IncrementInt (Variables|Default|GetClickCount)
    (:%20%20
      (CallFunction|ResetClickCount)
      (bind _returnvalue (CallFunction|CheckDoubleClick ClickActor))
      (return _returnvalue))))

(fn CheckDoubleClick
  (params (ClickActor :type Object%20Object%20Reference))
  (bind _clickcount (Variables|Default|GetClickCount))
  (Development|PrintString (Utilities|String|ToString(Integer) _clickcount))
  (return (and (== ClickActor (Variables|Default|GetClickObject)) (> _clickcount 1))))