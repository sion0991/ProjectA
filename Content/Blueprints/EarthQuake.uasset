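; EarthQuake is a skill actor: a traveling guard-break shockwave launched from the skill owner's weapon.
; OnSkill places it at the owner's Weapon_End socket with the owner's rotation.
; Tick moves it forward a fixed step per frame, independent of delta time, while tapering the Niagara SpawnNum parameter.
; Box overlaps apply negative-valued guard-break damage to each BP_Character not ignored, then add it to the Ignore list.
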(event OnComponentBeginOverlap(Box)
  (params (OverlappedComponent :type Primitive%20Component%20Object%20Reference) (OtherActor :type Actor%20Object%20Reference) (OtherComp :type Primitive%20Component%20Object%20Reference) (OtherBodyIndex :type Integer) (bFromSweep :type Boolean) (SweepResult :type Hit%20Result%20Structure%20%28by%20ref%29))
  (bind _asbp_character (Utilities|Casting|CastToBP_Character OtherActor))
  (if (not (CallFunction|IsIgnore _asbp_character))
    (Game|Damage|ApplyDamage _asbp_character -2e+01 (Pawn|GetController (Variables|Default|GetSkillOwner)) self "/Game/Blueprints/DamageType/DT_GuardBreakAttack.DT_GuardBreakAttack_C")
    (Utilities|Array|Add (Variables|Default|GetIgnore) _asbp_character)))

(event EventTick
  (params (DeltaSeconds :type Float%20%28single-precision%29))
  (Transformation|AddActorWorldOffset (* (Transformation|GetActorForwardVector) 1e+01))
  (Niagara|SetNiagaraVariable(Float) (Variables|Default|GetNiagara) "User.SpawnNum" (Variables|Default|GetSpawnNum))
  (Variables|Default|SetSpawnNum (Math|Float|Clamp(Float) (- (Variables|Default|GetSpawnNum) (* DeltaSeconds 0.2)))))

(fn ConstructionScript)

(fn OnSkill
  (bind _skillowner (Variables|Default|GetSkillOwner))
  (Transformation|SetActorTransform (Math|Transform|MakeTransform (Transformation|GetSocketLocation (Variables|/Script/Engine.Character|GetMesh _skillowner) "Weapon_End") (Transformation|GetActorRotation _skillowner))))