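; Status component for BP_Player that holds base stats and current HP, MP and SP.
; On BeginPlay it loads them from the StatusSlot save, or creates one with default stats.
; Helpers add or subtract stats, cap current values at maximums and total equipment bonuses into ItemStatus, though loading never runs that total.
; Timed buffs are unfinished, and SubStatus reverses the subtraction for HP, MP and AP.
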(event EventBeginPlay
  (Utilities|Casting|CastToBP_Player (Components|GetOwner))
  (CallFunction|LoadStatus))

(fn LoadStatus
  (bind _returnvalue (SaveGame|DoesSaveGameExist (Variables|Default|GetStatusSlot)))
  (if _returnvalue
    (bind _returnvalue_2 (SaveGame|LoadGamefromSlot (Variables|Default|GetStatusSlot)))
    (bind _assave_status (Utilities|Casting|CastToSave_Status _returnvalue_2))
    (bind _output_get (Variables|Default|SetSaveGame _assave_status))
    (bind (_stat _currenthp _currentmp _currentsp) (Default|Load _output_get))
    (Variables|Default|SetStatus _stat)
    (Variables|Default|SetCurrentHP _currenthp)
    (Variables|Default|SetCurrentMP _currentmp)
    (Variables|Default|SetCurrentSP _currentsp)
    (else
      (Development|PrintString "NotLoadStat")
      (CallFunction|SaveStatus))))

(fn SaveStatus
  (bind _returnvalue (SaveGame|DoesSaveGameExist (Variables|Default|GetStatusSlot)))
  (if _returnvalue
    (bind _returnvalue_2 (SaveGame|LoadGamefromSlot (Variables|Default|GetStatusSlot)))
    (bind _assave_status (Utilities|Casting|CastToSave_Status _returnvalue_2))
    (Development|PrintString "CoverStat")
    (Variables|Default|SetSaveGame _assave_status)
    (else
      (bind _returnvalue_3 (SaveGame|CreateSaveGameObject "/Game/Blueprints/Info/Save/Save_Status.Save_Status_C"))
      (Variables|Default|SetSaveGame _returnvalue_3)
      (Development|PrintString "NewSaveStat")
      (Variables|Default|SetStatus (Utilities|Struct|MakeST_Status 1e+02 1e+02 1e+02 5 5 5 5 5 5))))
  (Default|Save (Variables|Default|GetSaveGame) (Variables|Default|GetStatus) (Variables|Default|GetCurrentHP) (Variables|Default|GetCurrentMP) (Variables|Default|GetCurrentSP))
  (SaveGame|SaveGametoSlot (Variables|Default|GetSaveGame) (Variables|Default|GetStatusSlot)))

(fn AddStatus
  (params (Stat :type ST%20Status%20Structure))
  (Variables|Default|SetStatus (Utilities|Struct|MakeST_Status (+ (.hp Stat) (.hp (Variables|Default|GetStatus))) (+ (.mp Stat) (.mp (Variables|Default|GetStatus))) (+ (.ap Stat) (.ap (Variables|Default|GetStatus))) (+ (.atk (Variables|Default|GetStatus)) (.atk Stat)) (+ (.def (Variables|Default|GetStatus)) (.def Stat)) (+ (.str (Variables|Default|GetStatus)) (.str Stat)) (+ (.dex (Variables|Default|GetStatus)) (.dex Stat)) (+ (.int (Variables|Default|GetStatus)) (.int Stat)) (+ (.luck (Variables|Default|GetStatus)) (.luck Stat)))))

(fn SubStatus
  (params (Stat :type ST%20Status%20Structure))
  (Variables|Default|SetStatus (Utilities|Struct|MakeST_Status (- (.hp Stat) (.hp (Variables|Default|GetStatus))) (- (.mp Stat) (.mp (Variables|Default|GetStatus))) (- (.ap Stat) (.ap (Variables|Default|GetStatus))) (- (.atk (Variables|Default|GetStatus)) (.atk Stat)) (- (.def (Variables|Default|GetStatus)) (.def Stat)) (- (.str (Variables|Default|GetStatus)) (.str Stat)) (- (.dex (Variables|Default|GetStatus)) (.dex Stat)) (- (.int (Variables|Default|GetStatus)) (.int Stat)) (- (.luck (Variables|Default|GetStatus)) (.luck Stat)))))

(fn CalcCurrentStatus
  (params (Stat :type ST%20Status%20Structure))
  (Utilities|FlowControl|Sequence
    (:then_0
      (Variables|Default|SetCurrentHP (Math|Float|Min(Float) (+ (Variables|Default|GetCurrentHP) (.hp Stat)) (.HP (Utilities|Struct|BreakST_Status (Variables|Default|GetStatus))))))
    (:then_1
      (Variables|Default|SetCurrentMP (Math|Float|Min(Float) (+ (Variables|Default|GetCurrentMP) (.mp Stat)) (.MP (Utilities|Struct|BreakST_Status (Variables|Default|GetStatus))))))
    (:then_2
      (Variables|Default|SetCurrentSP (Math|Float|Min(Float) (+ (Variables|Default|GetCurrentSP) (.ap Stat)) (Utilities|Struct|BreakST_Status (Variables|Default|GetStatus)))))))

(fn CalcCurrentHP
  (params (Stat :type ST%20Status%20Structure))
  (Variables|Default|SetCurrentHP (Math|Float|Min(Float) (+ (Variables|Default|GetCurrentHP) (.hp Stat)) (.HP (Utilities|Struct|BreakST_Status (Variables|Default|GetStatus))))))

(fn CalcCurrentMP
  (params (Stat :type ST%20Status%20Structure))
  (Variables|Default|SetCurrentMP (Math|Float|Min(Float) (+ (Variables|Default|GetCurrentMP) (.mp Stat)) (.MP (Utilities|Struct|BreakST_Status (Variables|Default|GetStatus))))))

(fn CalcCurrentSP
  (params (Stat :type ST%20Status%20Structure))
  (Variables|Default|SetCurrentSP (Math|Float|Min(Float) (+ (Variables|Default|GetCurrentSP) (.ap Stat)) (Utilities|Struct|BreakST_Status (Variables|Default|GetStatus)))))

(fn DurationStatus
  (params (NewParam :type ST%20Status%20Structure) (NewParam1 :type Integer))
  (Development|PrintString "임시스텟올려야함")
  (Utilities|Time|SetTimerbyFunctionName self "SubStatus" (Math|Conversions|ToFloat(Integer) NewParam1)))

(fn CalcCurrentHPIndex
  (params (index :type Float%20%28double-precision%29))
  (bind _output_get (Variables|Default|SetCurrentHP (Math|Float|Min(Float) (+ (Variables|Default|GetCurrentHP) index) (.HP (Utilities|Struct|BreakST_Status (Variables|Default|GetStatus))))))
  (return (<= _output_get 0.0)))

(fn CalcCurrentMPIndex
  (params (index :type Float%20%28double-precision%29))
  (Variables|Default|SetCurrentMP (Math|Float|Min(Float) (+ (Variables|Default|GetCurrentMP) index) (.MP (Utilities|Struct|BreakST_Status (Variables|Default|GetStatus))))))

(fn CalcCurrentSPIndex
  (params (index :type Float%20%28double-precision%29))
  (Variables|Default|SetCurrentSP (Math|Float|Min(Float) (+ (Variables|Default|GetCurrentSP) index) (Utilities|Struct|BreakST_Status (Variables|Default|GetStatus)))))

(fn CalcItemStat
  (params (equips :type Array%20of%20BP%20Item%20Struct%20Structures))
  (Variables|Default|SetItemStatus (Utilities|Struct|MakeST_Status 0.0 0.0))
  (for _array_element equips
    (Variables|Default|SetItemStatus (Utilities|Struct|MakeST_Status (+ (.hp (Utilities|Struct|BreakBP_ItemStruct _array_element)) (.HP (Utilities|Struct|BreakST_Status (Variables|Default|GetItemStatus)))) (+ (.mp (Utilities|Struct|BreakBP_ItemStruct _array_element)) (.MP (Utilities|Struct|BreakST_Status (Variables|Default|GetItemStatus)))) (+ (.ap (Utilities|Struct|BreakBP_ItemStruct _array_element)) (.AP (Utilities|Struct|BreakST_Status (Variables|Default|GetItemStatus)))) (+ (.atk (Utilities|Struct|BreakBP_ItemStruct _array_element)) (.Atk (Utilities|Struct|BreakST_Status (Variables|Default|GetItemStatus)))) (+ (.def (Utilities|Struct|BreakBP_ItemStruct _array_element)) (.Def (Utilities|Struct|BreakST_Status (Variables|Default|GetItemStatus)))) (+ (.str (Utilities|Struct|BreakBP_ItemStruct _array_element)) (.Str (Utilities|Struct|BreakST_Status (Variables|Default|GetItemStatus)))) (+ (.dex (Utilities|Struct|BreakBP_ItemStruct _array_element)) (.Dex (Utilities|Struct|BreakST_Status (Variables|Default|GetItemStatus)))) (+ (.int (Utilities|Struct|BreakBP_ItemStruct _array_element)) (.Int (Utilities|Struct|BreakST_Status (Variables|Default|GetItemStatus)))) (+ (.luck (Utilities|Struct|BreakBP_ItemStruct _array_element)) (.Luck (Utilities|Struct|BreakST_Status (Variables|Default|GetItemStatus))))))))