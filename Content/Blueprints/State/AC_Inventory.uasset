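; Player inventory component that holds item and equipment slot arrays and mirrors changes to the main HUD widget.
; Items fill the first slot with a "None" index, and equip, unequip and swap functions move them between the arrays.
; Auto-equip maps item type to a slot, with weapons sharing one and rings choosing between two.
; Both arrays persist through a Save_Inventory save game, and loading refreshes the HUD and the player's visible equipment.
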(event EventBeginPlay
  (bind _asbp_player (Utilities|Casting|CastToBP_Player (Components|GetOwner)))
  (bind _output_get (Variables|Default|SetPlayer _asbp_player))
  (bind _asbp_pc (Utilities|Casting|CastToBP_PC (Pawn|GetController _output_get)))
  (Utilities|FlowControl|Delay 0.2)
  (Variables|Default|SetWidget (Variables|/Game/Blueprints/Gamplay/BP_PC.BP_PC_C|GetMainHUD _asbp_pc)))

(fn AddItem
  (params (Item :type BP%20Item%20Struct%20Structure))
  (bind (_array_element _array_index) (Utilities|Array|ForEachLoopwithBreak (Variables|Default|GetInventory) :!label _label)
    (:LoopBody
      (if (Utilities|Name|Equal(Name) (.ItemIndex (Utilities|Struct|BreakBP_ItemStruct _array_element)) "None")
        (Utilities|Array|SetArrayElem (Variables|Default|GetInventory) _array_index Item)
        (Default|SetItem (Variables|Default|GetWidget) _array_index)
        (goto _label Break)))))

(fn SubItem
  (params (NewParam1 :type Integer))
  (Utilities|Array|SetArrayElem :TargetArray (Variables|Default|GetInventory) :Index NewParam1)
  (Default|RemoveItem (Variables|Default|GetWidget) NewParam1))

(fn SaveInventory
  (bind _returnvalue (SaveGame|DoesSaveGameExist (Variables|Default|GetInventorySlot)))
  (if _returnvalue
    (bind _returnvalue_2 (SaveGame|LoadGamefromSlot (Variables|Default|GetInventorySlot)))
    (bind _assave_inventory (Utilities|Casting|CastToSave_Inventory _returnvalue_2))
    (Development|PrintString "CoverInv")
    (Variables|Default|SetSaveGame _assave_inventory)
    (else
      (bind _returnvalue_3 (SaveGame|CreateSaveGameObject "/Game/Blueprints/Info/Save/Save_Inventory.Save_Inventory_C"))
      (Variables|Default|SetSaveGame _returnvalue_3)
      (Development|PrintString "NewSaveInv")))
  (Default|Save (Variables|Default|GetSaveGame) (Variables|Default|GetInventory) (Variables|Default|GetEquipItems))
  (SaveGame|SaveGametoSlot (Variables|Default|GetSaveGame) (Variables|Default|GetInventorySlot)))

(fn LoadInventory
  (CallFunction|ItemUpdate (Variables|Default|GetInventorySlot))
  (bind _returnvalue (SaveGame|DoesSaveGameExist (Variables|Default|GetInventorySlot)))
  (if _returnvalue
    (bind _returnvalue_2 (SaveGame|LoadGamefromSlot (Variables|Default|GetInventorySlot)))
    (bind _assave_inventory (Utilities|Casting|CastToSave_Inventory _returnvalue_2))
    (bind _output_get (Variables|Default|SetSaveGame _assave_inventory))
    (Variables|Default|SetInventory (.Inventory (Default|Load _output_get)))
    (Variables|Default|SetEquipItems (.Equipments (Default|Load _output_get)))
    (Development|PrintString "LoadInv")
    (Default|LoadInventory (Variables|Default|GetWidget))
    (for (_array_element _array_index) (Variables|Default|GetEquipItems)
      (Default|ShowEquipment (Variables|Default|GetPlayer) _array_index))
    (else
      (Development|PrintString "NotLoadInv")
      (CallFunction|SaveInventory))))

(fn AutoEquipItem
  (params (index :type Integer))
  (bind _inventory (Variables|Default|GetInventory))
  (bind _output (Utilities|Array|Get(acopy) _inventory index))
  (bind _output_get (LocalVariables|SetEquipIndex (Utilities|Select :Index (.ItemType (Utilities|Struct|BreakBP_ItemStruct _output)) :NewEnumerator0 0 :NewEnumerator1 0 :NewEnumerator4 0 :NewEnumerator2 0 :NewEnumerator10 0 :NewEnumerator12 0 :NewEnumerator16 0 :NewEnumerator9 1 :NewEnumerator3 2 :NewEnumerator5 3 :NewEnumerator6 4 :NewEnumerator7 5 :NewEnumerator8 (Math|Integer|SelectInt 7 6 (Utilities|Array|IsValidIndex (Variables|Default|GetEquipItems) 6)) :NewEnumerator11 0 :NewEnumerator15 0)))
  (LocalVariables|SetTempItem (Utilities|Array|Get(acopy) (Variables|Default|GetEquipItems) _output_get))
  (Utilities|Array|SetArrayElem (Variables|Default|GetEquipItems) (LocalVariables|GetEquipIndex) _output)
  (Utilities|Array|SetArrayElem :TargetArray (Variables|Default|GetInventory) :Index index)
  (CallFunction|AddItem (LocalVariables|GetTempItem))
  (Default|SwapInventoryNEquip (Variables|Default|GetWidget) index (LocalVariables|GetEquipIndex))
  (return (LocalVariables|GetEquipIndex)))

(fn GetInvetoryItem
  (params (Index :type Integer))
  (return (Utilities|Array|Get(acopy) (Variables|Default|GetInventory) Index)))

(fn GetEquipItem
  (params (Index :type Integer))
  (return (Utilities|Array|Get(acopy) (Variables|Default|GetEquipItems) Index)))

(fn ClickUnEquipItem
  (params (Index :type Integer))
  (CallFunction|AddItem (Utilities|Array|Get(acopy) (Variables|Default|GetEquipItems) Index))
  (Utilities|Array|SetArrayElem :TargetArray (Variables|Default|GetEquipItems) :Index Index))

(fn DropUnEquipItem
  (params (EquipmentIndex :type Integer) (InventoryIndex :type Integer))
  (LocalVariables|SetTempItem (Utilities|Array|Get(acopy) (Variables|Default|GetInventory) InventoryIndex))
  (Utilities|Array|SetArrayElem (Variables|Default|GetInventory) InventoryIndex (Utilities|Array|Get(acopy) (Variables|Default|GetEquipItems) EquipmentIndex))
  (Utilities|Array|SetArrayElem (Variables|Default|GetEquipItems) EquipmentIndex (LocalVariables|GetTempItem))
  (Default|SwapInventoryNEquip (Variables|Default|GetWidget) InventoryIndex EquipmentIndex))

(fn SwapInventoryItem
  (params (From :type Integer) (To :type Integer))
  (Utilities|Array|Swap (Variables|Default|GetInventory) From To)
  (Default|SetItem (Variables|Default|GetWidget) From)
  (Default|SetItem (Variables|Default|GetWidget) To))

(fn EquipItem
  (params (InventoryIndex :type Integer) (EquipmentIndex :type Integer))
  (LocalVariables|SetTempItem (Utilities|Array|Get(acopy) (Variables|Default|GetEquipItems) EquipmentIndex))
  (Utilities|Array|SetArrayElem (Variables|Default|GetEquipItems) EquipmentIndex (Utilities|Array|Get(acopy) (Variables|Default|GetInventory) InventoryIndex))
  (Utilities|Array|SetArrayElem :TargetArray (Variables|Default|GetInventory) :Index InventoryIndex)
  (CallFunction|AddItem (LocalVariables|GetTempItem))
  (Default|SwapInventoryNEquip (Variables|Default|GetWidget) InventoryIndex EquipmentIndex)
  (return EquipmentIndex))